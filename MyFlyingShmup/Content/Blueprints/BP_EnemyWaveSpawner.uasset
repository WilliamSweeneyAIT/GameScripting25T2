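; BP_EnemyWaveSpawner spawns a wave of enemies defined in a wave data asset.
; On BeginPlay it validates the asset and starts the current wave on a timer after that wave's initial delay.
; StartWave loops over enemy members with per-member delays, spawning each and passing pickup-drop settings by message.
; The loop has no end check, and the wave ID never advances here.
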(event Custom|StartWave
  (Variables|Default|SetEnemyMemberIndex 0)
  (Utilities|FlowControl|Delay (.initialspawndelay (Utilities|Array|Get(acopy) (.enemymembers (Utilities|Array|Get(acopy) (Variables|/Game/Framework/PDA_SetOfWaves.PDA_SetOfWaves_C|GetSetOfWaves (Variables|Default|GetWaveDataAsset)) (Variables|Default|GetCurrentWaveID))) (Variables|Default|GetEnemyMemberIndex))) :!label _label)
  (bind _returnvalue (Game|SpawnActorfromClass (.enemyclass (Utilities|Array|Get(acopy) (.enemymembers (Utilities|Array|Get(acopy) (Variables|/Game/Framework/PDA_SetOfWaves.PDA_SetOfWaves_C|GetSetOfWaves (Variables|Default|GetWaveDataAsset)) (Variables|Default|GetCurrentWaveID))) (Variables|Default|GetEnemyMemberIndex))) (.spawntransform (Utilities|Array|Get(acopy) (.enemymembers (Utilities|Array|Get(acopy) (Variables|/Game/Framework/PDA_SetOfWaves.PDA_SetOfWaves_C|GetSetOfWaves (Variables|Default|GetWaveDataAsset)) (Variables|Default|GetCurrentWaveID))) (Variables|Default|GetEnemyMemberIndex))) "Undefined" "MultiplyWithRoot" 0 0))
  (Class|BPIMyFlyingShmup|AssignSpawnedEnemyProps(Message) _returnvalue (.shoulddroppickup (Utilities|Array|Get(acopy) (.enemymembers (Utilities|Array|Get(acopy) (Variables|/Game/Framework/PDA_SetOfWaves.PDA_SetOfWaves_C|GetSetOfWaves (Variables|Default|GetWaveDataAsset)) (Variables|Default|GetCurrentWaveID))) (Variables|Default|GetEnemyMemberIndex))) (.pickupclass (Utilities|Array|Get(acopy) (.enemymembers (Utilities|Array|Get(acopy) (Variables|/Game/Framework/PDA_SetOfWaves.PDA_SetOfWaves_C|GetSetOfWaves (Variables|Default|GetWaveDataAsset)) (Variables|Default|GetCurrentWaveID))) (Variables|Default|GetEnemyMemberIndex))))
  (Math|Integer|IncrementInt (Variables|Default|GetEnemyMemberIndex)
    (:%20%20
      (goto _label))))

(event EventBeginPlay
  (bind _wavedataasset (Variables|Default|GetWaveDataAsset)
    (:then
      (Utilities|Time|SetTimerbyEvent (delegate Custom|StartWave) (.initialwavedelay (Utilities|Array|Get(acopy) (Variables|/Game/Framework/PDA_SetOfWaves.PDA_SetOfWaves_C|GetSetOfWaves _wavedataasset) (Variables|Default|GetCurrentWaveID)))))
    (:else)))

(fn ConstructionScript)