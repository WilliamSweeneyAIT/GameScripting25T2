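; Bullet projectile Blueprint that damages actors it overlaps and then destroys itself.
; On overlap it runs the parent handler, then applies its Damage value to the other actor.
; A Piercing flag delays destruction by half a second, so further overlaps in that window also take damage; otherwise it is destroyed immediately.
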(event EventBeginPlay
  (|CallParentFunction) ; This node is disabled and will not be called.\nDrag off pins to build functionality.
)

(event Collision|EventActorBeginOverlap
  (params (OtherActor :type Actor%20Object%20Reference))
  (|CallParentFunction OtherActor)
  (Game|Damage|ApplyDamage OtherActor (Variables|Default|GetDamage) 0 0)
  (if (Variables|Default|GetPiercing)
    (Utilities|FlowControl|Delay 0.5))
  (Actor|DestroyActor))

(fn ConstructionScript
  (|CallParentFunction))