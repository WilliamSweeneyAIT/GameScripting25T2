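; Enemy boss Blueprint that moves itself into the play area when play begins.
; EnterPlayArea drives an X offset from a timeline, while MoveSideToSide, not called in this file, drives a slowed Y offset.
; Both feed the captured start location plus the scaled curve value into a swept AddActorWorldOffset each update, so movement accumulates rather than setting an absolute position.
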(event Custom|EnterPlayArea
  (Variables|Default|SetInitialLocation (Transformation|GetActorLocation))
  (bind _x_offset (Timeline|TL_EnterPlayArea PlayFromStart)
    (:Update
      (Transformation|AddActorWorldOffset (+ (Variables|Default|GetInitialLocation) (Math|Vector|MakeVector (* _x_offset 1e+03) 0.0 0.0)) true))))

(event Custom|MoveSideToSide
  (Variables|Default|SetInitialLocation (Transformation|GetActorLocation))
  (Components|Timeline|SetPlayRate (Variables|Default|GetTL_MoveSideToSide) 0.05)
  (bind _y_value (Timeline|TL_MoveSideToSide PlayFromStart)
    (:Update
      (Transformation|AddActorWorldOffset (+ (Variables|Default|GetInitialLocation) (Math|Vector|MakeVector 0.0 (* _y_value 4e+03) 0.0)) true))))

(event EventBeginPlay
  (|CallParentFunction)
  (CallFunction|EnterPlayArea))

(event Collision|EventActorBeginOverlap
  (params (OtherActor :type Actor%20Object%20Reference))
  (|CallParentFunction OtherActor) ; This node is disabled and will not be called.\nDrag off pins to build functionality.
)

(event EventTick
  (params (DeltaSeconds :type Float%20%28single-precision%29)))

(fn ConstructionScript
  (|CallParentFunction))