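; Base enemy actor that tracks health, shows it on a widget health bar, and deals fixed damage to any actor it overlaps.
; Incoming damage updates the bar; surviving hits play a sound and briefly flash an overlay material on the mesh.
; Death triggers camera shake and adds max health to score via the player controller, spawns an explosion and optional pickup, then destroys the actor.
; An event lets the pickup drop be assigned after spawning.
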(event Custom|ApplyDamage
  (params (Damage :type Float%20%28double-precision%29))
  ;[0.15 0.15 0.15 0.5] Set progress bar of widget (Health bar) to current health.
  (Variables|Default|SetHealth (- (Variables|Default|GetHealth) Damage))
  (bind _aswbp_enemy_health_bar (Utilities|Casting|CastToWBP_EnemyHealthBar (UserInterface|GetUserWidgetObject (Variables|Default|GetWidget))))
  (Default|SetHealth _aswbp_enemy_health_bar (/ (Variables|Default|GetHealth) (Variables|Default|GetMaxHealth))))

(event EventBeginPlay
  (Variables|Default|SetHealth (Variables|Default|GetMaxHealth)))

(event Collision|EventActorBeginOverlap
  (params (OtherActor :type Actor%20Object%20Reference))
  (Game|Damage|ApplyDamage OtherActor 5e+01 0 0))

(event Game|Damage|EventAnyDamage
  (params (Damage :type Float%20%28single-precision%29) (DamageType :type Damage%20Type%20Object%20Reference) (InstigatedBy :type Controller%20Object%20Reference) (DamageCauser :type Actor%20Object%20Reference))
  (CallFunction|ApplyDamage Damage)
  ;[0.15 0.15 0.15 0.5] Check for Enemy health = 0. If true, trigger death.
  (if (<= (Variables|Default|GetHealth) 0.0)
    ;[0.15 0.15 0.15 0.5] Camera Shake and Enemy Destruction
    (Development|PrintString "Enemy has died!")
    (Audio|PlaySound2D "/Game/SoundFX/Explosion.Explosion" 2.5 1.0 0.3 0 0)
    (Utilities|FlowControl|Sequence
      (:then_0
        (bind _asmy_player_controller (Utilities|Casting|CastTomyPlayerController (Game|GetPlayerController 0)))
        (Default|ApplyCameraShake _asmy_player_controller)
        (Default|AddtoScore _asmy_player_controller (Variables|Default|GetMaxHealth)))
      (:then_1
        (Game|SpawnActorfromClass "/Game/Particles/BP_EnemyDeathExplosion.BP_EnemyDeathExplosion_C" (Math|Transform|MakeTransform (Transformation|GetActorLocation) "0, 0, 0" "1.000000,1.000000,1.000000") "AlwaysSpawn" "MultiplyWithRoot" 0 0)
        (if (Variables|Default|GetSpawn%20Pick%20Up%20on%20Death)
          (Game|SpawnActorfromClass (Variables|Default|GetPick%20Up%20Type%20to%20Spawn) (Transformation|GetActorTransform) "AlwaysSpawn" "MultiplyWithRoot" 0 0.0 0)))
      (:then_2
        (Actor|DestroyActor)))
    (else
      ;[0.15 0.15 0.15 0.5] Damage feedback (Visual and sound)
      (Audio|PlaySound2D "/Game/SoundFX/HitSound.HitSound" 1.0 1.0 0.0 0 0)
      (for _array_element (Utilities|Array|MakeArray (Actor|GetComponentbyClass "/Script/Engine.StaticMeshComponent"))
        (Rendering|Material|SetOverlayMaterial _array_element "/Game/Materials/M_DamageFlash.M_DamageFlash" :!class /Script/Engine.MeshComponent))
      (Utilities|FlowControl|Delay 0.2)
      (for _array_element_2 (Utilities|Array|MakeArray (Actor|GetComponentbyClass "/Script/Engine.StaticMeshComponent"))
        (Rendering|Material|SetOverlayMaterial _array_element_2 0 :!class /Script/Engine.MeshComponent)))))

(event EventAssignSpawnedEnemyProps
  (params (SpawnPickUpOnDeath :type Boolean) (PickUpTypeToSpawn :type BP%20Base%20Pickup%20Class%20Reference))
  (Variables|Default|SetSpawn%20Pick%20Up%20on%20Death SpawnPickUpOnDeath)
  (Variables|Default|SetPick%20Up%20Type%20to%20Spawn PickUpTypeToSpawn))

(fn ConstructionScript)