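; BP_Enemy_Shotgunner is a short-lived enemy that fires three-bullet volleys and destroys itself eight seconds after BeginPlay.
; Tick turns its root in yaw only to face the player pawn.
; A looping timer calls ShootBullet, which spawns BP_EnemyBullet at three spawn points with a 2D fire sound.
; ShootBullet also re-triggers itself through a short Delay, so rapid volleys continue after the timer first fires.
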(event Custom|ShootBullet
  (Game|SpawnActorfromClass "/Game/Blueprints/BP_EnemyBullet.BP_EnemyBullet_C" (Transformation|GetWorldTransform (Variables|Default|GetBulletSpawnPoint_0)) "Undefined" "MultiplyWithRoot" 0 0 :!label _label)
  (Game|SpawnActorfromClass "/Game/Blueprints/BP_EnemyBullet.BP_EnemyBullet_C" (Transformation|GetWorldTransform (Variables|Default|GetBulletSpawnPoint_1)) "Undefined" "MultiplyWithRoot" 0 0)
  (Game|SpawnActorfromClass "/Game/Blueprints/BP_EnemyBullet.BP_EnemyBullet_C" (Transformation|GetWorldTransform (Variables|Default|GetBulletSpawnPoint_2)) "Undefined" "MultiplyWithRoot" 0 0)
  (Audio|PlaySound2D "/Game/SoundFX/EnemyFire.EnemyFire" 1.5 1.0 0.0 0 0)
  (Utilities|FlowControl|Delay 0.7)
  (goto _label))

(event EventBeginPlay
  (Utilities|Time|SetTimerbyEvent (delegate Custom|ShootBullet) 3.5 true true)
  (Utilities|FlowControl|Delay 8.0)
  (Actor|DestroyActor))

(event EventTick
  (params (DeltaSeconds :type Float%20%28single-precision%29))
  (Transformation|SetWorldRotation (Variables|Default|GetDefaultSceneRoot) (Math|Rotator|MakeRotator 0.0 0.0 (.yaw (Math|Rotator|FindLookatRotation (Transformation|GetActorLocation) (Transformation|GetActorLocation (Game|Player|GetPlayerPawn 0))))) false false))

(fn ConstructionScript)